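; BP_Character is a character Blueprint with a configurable top-down camera and a key-triggered camera shake.
; The construction script sets the CameraBoom arm length, relative rotation, lag toggle and lag speed from the Blueprint's variables.
; Pressing F calls CameraShakeEvent, which plays BP_ShakeCamera as a world camera shake centred on the top-down camera's location with a small outer radius.
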(event `Key|F`
  (params (Key :type "Key Structure"))
  (:`Pressed`
    (`self.CameraShakeEvent`)))

(fn `CameraShakeEvent`
  (`GameplayStatics.PlayWorldCameraShake` "/Game/Blueprint/Game/BP_ShakeCamera.BP_ShakeCamera_C" (`SceneComponent.K2_GetComponentLocation` (`self.TopDownCameraComponent`)) 0.0 30.0))

(fn `UserConstructionScript`
  (bind _cameraboom (`self.CameraBoom`))
  (set `SpringArmComponent.TargetArmLength` (`self.CameraHeightMax`) _cameraboom)
  (`SceneComponent.K2_SetRelativeRotation` _cameraboom (`self.RotatorCamera`) false false)
  (set `SpringArmComponent.bEnableCameraLag` (`self.Flow`) _cameraboom)
  (set `SpringArmComponent.CameraLagSpeed` (`self.CoefficientSmooth`) _cameraboom))