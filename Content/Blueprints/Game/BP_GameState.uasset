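; Game state for a top-down shooter that tracks lives, score, phase progression and victory.
; On BeginPlay it reads the current level's final phase and score thresholds from DT_Levels.
; Added points advance the phase and enemy wave index past each threshold, pausing on an end-game screen at the final phase.
; Respawn and enemy spawn queries update lives and enemy counts on the HUD's gameplay widget and return phase data.
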(event `self.ReceiveBeginPlay`
  (set `self.Lives` (`self.MaxLives`))
  (bind _returnvalue (`GameplayStatics.GetCurrentLevelName` true))
  (bind _outrownames (`DataTableFunctionLibrary.GetDataTableRowNames` "/Game/Tables/Menu/DT_Levels.DT_Levels"))
  (for _array_element _outrownames
    (bind _returnvalue_2 (`|GetDataTableRow` "/Game/Tables/Menu/DT_Levels.DT_Levels" _array_element)
      (:`then`
        (bind (_levelname _finalphase _phasewinscore) (break `/Game/Tables/Menu/S_Levels` _returnvalue_2))
        (if (== _levelname (`KismetStringLibrary.Conv_StringToName` _returnvalue))
          (set `self.Final Phase` _finalphase)
          (bind _output_get (set `self.Phase Win Score` _phasewinscore))
          (break)))))
  (set `self.CurrentEnemyWaveIndex` 0)
  (set `self.CurrentPhaseScore` (`|GetArrayItem` _output_get)))

(fn `AddPoints`
  (params (PointsToAdd :type Integer))
  (bind _output_get (set `self.PlayerScore` (+ PointsToAdd (`self.PlayerScore`))))
  (bind _aswbp_gameplay (`self.Get_WBPGameplayWidget`))
  (bind _wbp_stats (`/Game/Blueprints/UI/WBP_Gameplay.WBP_Stats` _aswbp_gameplay))
  (`/Game/Blueprints/UI/Stats/WBP_Stats.SetScore` _wbp_stats _output_get)
  (`/Game/Blueprints/UI/Stats/WBP_Stats.EnemiesChanged` _wbp_stats (`self.EnemiesLeft`))
  (for (_array_element _array_index) (`self.Phase Win Score`)
    (if (< (`self.PlayerScore`) _array_element)
      (set `self.CurrentPhaseScore` _array_element)
      (break)
      (else
        (bind _returnvalue (select `int` _array_index :`0` "NewEnumerator1" :`1` "NewEnumerator2" :`2` "NewEnumerator3" :`3` "NewEnumerator4" :!type "/Game/Blueprints/SaveGame/CheckPoint/E_PhaseLevel Enum"))
        (bind _output_get_2 (set `self.CurrentPhase` _returnvalue))
        (set `self.CurrentEnemyWaveIndex` (select `int` _array_index :`0` 1 :`1` 2 :`2` 3))
        (`/Game/Blueprints/UI/Stats/WBP_Stats.PhaseChanged` _wbp_stats _output_get_2)
        (bind _returnvalue_2 (`|EnumEquality` _returnvalue (`self.Final Phase`)))
        (if _returnvalue_2
          (`self.PlayerWins` _returnvalue_2))))))

(fn `CanPlayerRespawn`
  (returns (bCanPlayerRespawn :type Boolean) (CurrentPhase :type "/Game/Blueprints/SaveGame/CheckPoint/E_PhaseLevel Enum"))
  (bind _lives (`self.Lives`))
  (bind _aswbp_gameplay (`self.Get_WBPGameplayWidget`))
  (`/Engine/EditorBlueprintResources/StandardMacros.DecrementInt` _lives
    (:`  `
      (`/Game/Blueprints/UI/Stats/WBP_Stats.LivesChanged` (`/Game/Blueprints/UI/WBP_Gameplay.WBP_Stats` _aswbp_gameplay) _lives)
      (return (> _lives 0) (`self.CurrentPhase`)))))

(fn `Get_WBPGameplayWidget`
  (returns (`AsWBP Gameplay` :type "/Game/Blueprints/UI/WBP_Gameplay Object Reference"))
  (bind _asbp_tdsplayer_controller (cast `/Game/Blueprints/Game/BP_TDSPlayerController` (`GameplayStatics.GetPlayerController` 0)))
  (bind _asbp_tdshud (cast `/Game/Blueprints/UI/BP_TDSHUD` (`PlayerController.GetHUD` _asbp_tdsplayer_controller)))
  (bind _aswbp_gameplay (cast `/Game/Blueprints/UI/WBP_Gameplay` (`TDS_HUD.GetGameplayWidget` _asbp_tdshud)))
  (return _aswbp_gameplay))

(fn `GetEnemyPhase`
  (params (NumberOfSpawnedEnemies :type Integer))
  (returns (CurrentPhase :type "/Game/Blueprints/SaveGame/CheckPoint/E_PhaseLevel Enum") (CurrentPhaseScore :type Integer) (CurrentEnemyWaveIndex :type Integer))
  (set `self.EnemiesLeft` NumberOfSpawnedEnemies)
  (bind _aswbp_gameplay (`self.Get_WBPGameplayWidget`))
  (`/Game/Blueprints/UI/Stats/WBP_Stats.EnemiesChanged` (`/Game/Blueprints/UI/WBP_Gameplay.WBP_Stats` _aswbp_gameplay) (`self.EnemiesLeft`))
  (return (`self.CurrentPhase`) (`self.CurrentPhaseScore`) (`self.CurrentEnemyWaveIndex`)))

(fn `PlayerWins`
  (params (bIsWin :type Boolean))
  (bind _returnvalue (`GameplayStatics.GetPlayerController` 0))
  (bind _endgamemenuref (`self.EndGameMenuRef`))
  (bind _returnvalue_2 (`|CreateWidget` "/Game/Blueprints/UI/Menu/WBP_EndGame.WBP_EndGame_C" null bIsWin))
  (set `self.EndGameMenuRef` _returnvalue_2)
  (if (`GameplayStatics.IsGamePaused`)
    (`Widget.RemoveFromParent` _endgamemenuref)
    (`GameplayStatics.SetGamePaused` false)
    (set `PlayerController.bShowMouseCursor` false _returnvalue)
    (`WidgetBlueprintLibrary.SetInputMode_GameOnly` _returnvalue)
    (else
      (`UserWidget.AddToViewport` _endgamemenuref 0)
      (`GameplayStatics.SetGamePaused` true)
      (set `PlayerController.bShowMouseCursor` true _returnvalue)
      (`WidgetBlueprintLibrary.SetInputMode_GameAndUIEx` _returnvalue (`self.EndGameMenuRef`) "LockInFullscreen" false))))

(fn `UserConstructionScript`)