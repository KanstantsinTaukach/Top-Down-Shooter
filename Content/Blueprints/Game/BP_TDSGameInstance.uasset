(event `self.HandleNetworkError`
  (params (FailureType :type "ENetworkFailure Enum" :default "NetDriverAlreadyExists") (bIsServer :type Boolean))
  (`KismetSystemLibrary.PrintString` (`KismetStringLibrary.Concat_StrStr` "Network Error: " (`|GetEnumeratorNameAsString` FailureType)) true true (struct :`R` 0.323143 :`G` 0.003347 :`A` 1.0) 10.0))

(event `self.HandleTravelError`
  (params (FailureType :type "ETravelFailure Enum" :default "NoLevel"))
  (`KismetSystemLibrary.PrintString` (`KismetStringLibrary.Concat_StrStr` "Travel Error: " (`|GetEnumeratorNameAsString` FailureType)) true true (struct :`R` 0.323143 :`G` 0.003347 :`A` 1.0) 10.0))

(event `LaunchLobbyEvent`
  (params (MaxPlayers :type Integer) (bUseLAN :type Boolean))
  (`CreateSessionCallbackProxy.CreateSession` (`GameplayStatics.GetPlayerController` 0) MaxPlayers bUseLAN
    (:`OnSuccess`
      (`GameplayStatics.OpenLevel` "LobbyLevel" true "?listen"))
    (:`OnFailure`
      (`KismetSystemLibrary.PrintString` "Failed create session" true true (struct :`R` 1.0 :`A` 1.0) 10.0))))

(event `/Game/Blueprints/Game/Lobby/BPI_NetworkInterface.CreateSession`
  (params (MaxPlayers :type Integer) (bIsLan :type Boolean))
  ;[1 1 1] BPI_NetworkInterface
  (`self.LaunchLobbyEvent` MaxPlayers bIsLan))

(event `/Game/Blueprints/Game/Lobby/BPI_NetworkInterface.JoinSession`
  (params (SearchResult :type "BlueprintSessionResult Structure (by ref)"))
  ;[1 1 1] BPI_NetworkInterface
  (`self.JoinSessionEvent` SearchResult))

(event `JoinSessionEvent`
  (params (SearchResult :type "BlueprintSessionResult Structure (by ref)"))
  (`JoinSessionCallbackProxy.JoinSession` (`GameplayStatics.GetPlayerController` 0) SearchResult
    (:`OnFailure`
      (`KismetSystemLibrary.PrintString` "Failed join session" true true (struct :`R` 1.0 :`A` 1.0) 10.0))))