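; Player controller for the main menu that sets up the menu screen and restores saved audio settings.
; On BeginPlay for the local player, it points the view at a level CameraActor, creates the main menu widget and shows the mouse cursor.
; It activates the base sound mix, then applies effects and music volumes from the AudioSettings save slot as sound class overrides, if that save exists.
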(event `self.ReceiveBeginPlay`
  (bind _returnvalue (`GameplayStatics.GetPlayerController` 0))
  (if (`self.IsLocalPlayerController`)
    (bind _returnvalue_2 (`GameplayStatics.GetActorOfClass` "/Script/Engine.CameraActor"))
    (`self.SetViewTargetWithBlend` _returnvalue _returnvalue_2 0.0 "VTBlend_Linear" 0.0 false)
    (`GameplayStatics.SetBaseSoundMix` "/Game/Sounds/SoundClasses/Mix_TDSMain.Mix_TDSMain")
    (bind _returnvalue_3 (`|CreateWidget` "/Game/Blueprints/UI/Menu/WBP_MainMenu.WBP_MainMenu_C" _returnvalue))
    (`UserWidget.AddToViewport` _returnvalue_3 0)
    (set `PlayerController.bShowMouseCursor` true _returnvalue)
    (bind _returnvalue_4 (`GameplayStatics.DoesSaveGameExist` "AudioSettings"))
    (if _returnvalue_4
      (bind _returnvalue_5 (`GameplayStatics.LoadGameFromSlot` "AudioSettings"))
      (bind _asbp_save_game (cast `/Game/Blueprints/SaveGame/BP_SaveGame` _returnvalue_5))
      (bind _output_get (set `self.As BP Save Game` _asbp_save_game))
      (`GameplayStatics.SetSoundMixClassOverride` "/Game/Sounds/SoundClasses/Mix_TDSMain.Mix_TDSMain" "/Game/Sounds/SoundClasses/TDSEffectsClass.TDSEffectsClass" (`/Game/Blueprints/SaveGame/BP_SaveGame.EffectsSound` _output_get))
      (`GameplayStatics.SetSoundMixClassOverride` "/Game/Sounds/SoundClasses/Mix_TDSMain.Mix_TDSMain" "/Game/Sounds/SoundClasses/TDSMusicClass.TDSMusicClass" (`/Game/Blueprints/SaveGame/BP_SaveGame.MusicSound` _output_get)))))

(fn `UserConstructionScript`)