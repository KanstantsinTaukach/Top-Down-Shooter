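; Lobby game state that tracks which player colors are taken and reports which remain free.
; Server-side events add, remove or swap entries in BlockColors as color selections change.
; After each change it loops the lobby game mode's player controllers and sends each the blocked list through UpdateColorsInLobbyOnClient.
; GetAvailableColors filters AllColors against the blocked list, and GetBlockColors returns that list.
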(event `SelectedNewColor_OnServer`
  (params (RemoveColor :type "MaterialInstance Object Reference") (AddColor :type "MaterialInstance Object Reference"))
  (bind _blockcolors (`self.BlockColors`))
  (`KismetArrayLibrary.Array_RemoveItem` _blockcolors RemoveColor)
  (`KismetArrayLibrary.Array_Add` _blockcolors AddColor)
  (bind _asbp_lobby_game_mode (cast `/Game/Blueprints/Game/Lobby/BP_LobbyGameMode` (`GameplayStatics.GetGameMode`)))
  (for _array_element (`/Game/Blueprints/Game/Lobby/BP_LobbyGameMode.PlayerControllers` _asbp_lobby_game_mode)
    (bind _asbp_lobby_player_controller (cast `/Game/Blueprints/Game/Lobby/BP_LobbyPlayerController` _array_element))
    (`/Game/Blueprints/Game/Lobby/BP_LobbyPlayerController.UpdateColorsInLobby_OnClient` _asbp_lobby_player_controller (`self.BlockColors`))))

(event `AddOrRemoveColorToBlock_OnServer`
  (params (Color :type "MaterialInstance Object Reference") (bIsRemove :type Boolean))
  (bind _blockcolors (`self.BlockColors`))
  (if bIsRemove
    (`KismetArrayLibrary.Array_RemoveItem` _blockcolors Color)
    (else
      (`KismetArrayLibrary.Array_Add` _blockcolors Color)))
  (bind _asbp_lobby_game_mode (cast `/Game/Blueprints/Game/Lobby/BP_LobbyGameMode` (`GameplayStatics.GetGameMode`)))
  (for _array_element (`/Game/Blueprints/Game/Lobby/BP_LobbyGameMode.PlayerControllers` _asbp_lobby_game_mode)
    (bind _asbp_lobby_player_controller (cast `/Game/Blueprints/Game/Lobby/BP_LobbyPlayerController` _array_element))
    (`/Game/Blueprints/Game/Lobby/BP_LobbyPlayerController.UpdateColorsInLobby_OnClient` _asbp_lobby_player_controller (`self.BlockColors`))))

(fn `GetAvailableColors`
  (returns (AvailableColorsOut :type "Array of MaterialInstance Object Reference"))
  (locals (AvailableColors :type "Array of MaterialInstance Object Reference") (bIsBlocked :type Boolean))
  (for _array_element (`self.AllColors`)
    (if (> (`KismetArrayLibrary.Array_Length` (`self.BlockColors`)) 0)
      (set `local.bIsBlocked` false)
      (for _array_element_2 (`self.BlockColors`)
        (if (== _array_element_2 _array_element)
          (set `local.bIsBlocked` true)))
      (if (not (`local.bIsBlocked`))
        (`KismetArrayLibrary.Array_Add` (`local.AvailableColors`) _array_element))
      (else
        (`KismetArrayLibrary.Array_Add` (`local.AvailableColors`) _array_element))))
  (return (`local.AvailableColors`)))

(fn `GetBlockColors`
  (returns (BlockColorsOut :type "Array of MaterialInstance Object Reference"))
  (locals (bCanTake :type Boolean) (AvailableColors :type "Array of MaterialInterface Object Reference"))
  (return (`self.BlockColors`)))

(fn `UserConstructionScript`)