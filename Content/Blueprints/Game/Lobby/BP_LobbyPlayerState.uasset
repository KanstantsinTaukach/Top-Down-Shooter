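; Lobby player state that passes the player's name to its controller and exposes queries for blocked and available colors.
; On BeginPlay it casts its owner to BP_LobbyPlayerController and calls UpdatePlayerName.
; GetAbailableColors filters AllColors against BlockedColors, while GetBlockedColors returns the blocked list directly.
; The server events for selecting a color and editing the blocked list are empty stubs.
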(event `SelectedNewColor_OnServer`)

(event `AddOrRemoveColorToBlock_OnServer`
  (params (Color :type "MaterialInstance Object Reference") (IsRemove :type Boolean)))

(event `self.ReceiveBeginPlay`
  (bind _asbp_lobby_player_controller (cast `/Game/Blueprints/Game/Lobby/BP_LobbyPlayerController` (`self.GetOwner`)))
  (`/Game/Blueprints/Game/Lobby/BP_LobbyPlayerController.UpdatePlayerName` _asbp_lobby_player_controller (`KismetTextLibrary.Conv_StringToText` (`self.GetPlayerName`))))

(fn `GetAbailableColors`
  (returns (AvailableColors :type "Array of MaterialInstance Object Reference"))
  (locals (IsAbailable :type Boolean) (AllAvailableColors :type "Array of MaterialInstance Object Reference"))
  (for _array_element (`self.AllColors`)
    (set `local.IsAbailable` true)
    (for _array_element_2 (`self.BlockedColors`)
      (if (== _array_element_2 _array_element)
        (set `local.IsAbailable` false)
        (break)))
    (if (`local.IsAbailable`)
      (`KismetArrayLibrary.Array_Add` (`local.AllAvailableColors`) _array_element)))
  (return (`local.AllAvailableColors`)))

(fn `GetBlockedColors`
  (returns (BlockedColors :type "Array of MaterialInstance Object Reference"))
  (return (`self.BlockedColors`)))

(fn `UserConstructionScript`)