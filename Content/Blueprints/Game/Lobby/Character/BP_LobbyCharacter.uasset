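; BP_LobbyCharacter is the lobby character, showing a player's chosen color and ready state.
; A server event forwards color changes to a multicast, which stores CharacterColor and applies it as the skeletal mesh's first material.
; On BeginPlay, remote instances reapply the stored color.
; A ready multicast plays a rifle ironsights idle montage on the mesh.
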(event `ChangeColor_OnServer`
  (params (CharacterColor :type "MaterialInstance Object Reference"))
  (`self.ChangeColor_Multicast` CharacterColor))

(event `ChangeColor_Multicast`
  (params (CharacterColor :type "MaterialInstance Object Reference"))
  (bind _output_get (set `self.CharacterColor` CharacterColor))
  (`PrimitiveComponent.SetMaterial` (`self.SkeletalMesh_Character`) 0 _output_get))

(event `self.ReceiveBeginPlay`
  (`/Engine/EditorBlueprintResources/ActorMacros.Switch Has Authority`
    (:`Remote`
      (`PrimitiveComponent.SetMaterial` (`self.SkeletalMesh_Character`) 0 (`self.CharacterColor`)))))

(event `IAmReady_Multicast`
  (`|PlayMontage` (`self.SkeletalMesh_Character`) "/Game/Blueprints/Character/Mannequin/Animations/TDSAnimations/AM_TDS_Idle_Rifle_Ironsights.AM_TDS_Idle_Rifle_Ironsights"))

(fn `UserConstructionScript`)