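; Lobby game mode that seats joining players at target points, manages their character colors and launches the selected level.
; PostLogin claims a free TargetPoint, spawns a lobby character there and assigns a random available color; logout frees both.
; Color changes update the blocked-color list in BP_LobbyGameState, and level selections are pushed to each controller's lobby widget.
; Player colors can be saved to the game instance by PlayerId, and LaunchGame uses seamless server travel.
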(event `LaunchGame`
  (params (LevelName :type String))
  (`Types.SeamlessServerTravel` self LevelName))

(event `UpdateLevelName`
  (params (SelectedLevel :type Name))
  (bind _output_get (set `self.SelectedLevel` SelectedLevel))
  (for _array_element (`self.PlayerControllers`)
    (bind _asbp_lobby_player_controller (cast `/Game/Blueprints/Game/Lobby/BP_LobbyPlayerController` _array_element))
    (`/Game/Blueprints/Game/Lobby/BP_LobbyPlayerController.UpdateLobbyWidgetOnClient` _asbp_lobby_player_controller _output_get)))

(event `self.K2_PostLogin`
  (params (NewPlayer :type "PlayerController Object Reference"))
  (bind _targetpoints (`self.TargetPoints`))
  (bind _keys (`BlueprintMapLibrary.Map_Keys` (`self.TargetPoints`)))
  (if (not (> (`KismetArrayLibrary.Array_Length` _keys) 0))
    (bind _outactors (`GameplayStatics.GetAllActorsOfClass` "/Script/Engine.TargetPoint"))
    (for _array_element _outactors
      (`BlueprintMapLibrary.Map_Add` (`self.TargetPoints`) _array_element)))
  (bind _asbp_lobby_player_controller (cast `/Game/Blueprints/Game/Lobby/BP_LobbyPlayerController` NewPlayer))
  (`KismetArrayLibrary.Array_Add` (`self.PlayerControllers`) _asbp_lobby_player_controller)
  (set `/Game/Blueprints/Game/Lobby/BP_LobbyPlayerController.CurrentLevelByServer` (`self.SelectedLevel`) _asbp_lobby_player_controller)
  (bind _keys_2 (`BlueprintMapLibrary.Map_Keys` _targetpoints))
  (for _array_element_2 _keys_2
    (if (not (`BlueprintMapLibrary.Map_Find` _targetpoints _array_element_2))
      (`BlueprintMapLibrary.Map_Add` _targetpoints _array_element_2 true)
      (bind _returnvalue (`|SpawnActorFromClass` "/Game/Blueprints/Game/Lobby/Character/BP_LobbyCharacter.BP_LobbyCharacter_C" (`self.GetTransform` _array_element_2) "AlwaysSpawn" "OverrideRootScale" null null))
      (set `/Game/Blueprints/Game/Lobby/BP_LobbyPlayerController.OccupiedPoint` _array_element_2 _asbp_lobby_player_controller)
      (`/Game/Blueprints/Game/Lobby/BP_LobbyPlayerController.SaveLobbyCharacter` _asbp_lobby_player_controller _returnvalue)
      (`self.SetRandomCharacterColor` _asbp_lobby_player_controller)
      (break))))

(event `self.K2_OnLogout`
  (params (ExitingController :type "Controller Object Reference"))
  (bind _asbp_lobby_player_controller (cast `/Game/Blueprints/Game/Lobby/BP_LobbyPlayerController` ExitingController))
  (`KismetArrayLibrary.Array_RemoveItem` (`self.PlayerControllers`) _asbp_lobby_player_controller)
  (`BlueprintMapLibrary.Map_Add` (`self.TargetPoints`) (`/Game/Blueprints/Game/Lobby/BP_LobbyPlayerController.OccupiedPoint` _asbp_lobby_player_controller))
  (bind _asbp_lobby_game_state (cast `/Game/Blueprints/Game/Lobby/BP_LobbyGameState` (`GameplayStatics.GetGameState`)))
  (`/Game/Blueprints/Game/Lobby/BP_LobbyGameState.AddOrRemoveColorToBlock_OnServer` _asbp_lobby_game_state (`/Game/Blueprints/Game/Lobby/Character/BP_LobbyCharacter.CharacterColor` (`/Game/Blueprints/Game/Lobby/BP_LobbyPlayerController.LobbyCharacter` _asbp_lobby_player_controller)) true))

(event `SaveColorForPlayers`
  (bind _asbp_tdsgame_instance (cast `/Game/Blueprints/Game/BP_TDSGameInstance` (`GameplayStatics.GetGameInstance`)))
  (for _array_element (`self.PlayerControllers`)
    (bind _asbp_lobby_player_controller (cast `/Game/Blueprints/Game/Lobby/BP_LobbyPlayerController` _array_element))
    (`BlueprintMapLibrary.Map_Add` (`/Game/Blueprints/Game/BP_TDSGameInstance.ColorForPlayers` _asbp_tdsgame_instance) (`KismetStringLibrary.Conv_IntToString` (`PlayerState.PlayerId` (`Controller.PlayerState` _asbp_lobby_player_controller))) (`/Game/Blueprints/Game/Lobby/Character/BP_LobbyCharacter.CharacterColor` (`/Game/Blueprints/Game/Lobby/BP_LobbyPlayerController.LobbyCharacter` _asbp_lobby_player_controller)))
    (`/Game/Blueprints/Game/Lobby/BP_LobbyPlayerController.RemoveAllWidget` _asbp_lobby_player_controller)))

(event `UpdateColorForCharacter`
  (params (Material :type "MaterialInstance Object Reference") (Controller :type "/Game/Blueprints/Game/Lobby/BP_LobbyPlayerController Object Reference"))
  (bind _asbp_lobby_game_state (cast `/Game/Blueprints/Game/Lobby/BP_LobbyGameState` (`GameplayStatics.GetGameState`)))
  (`/Game/Blueprints/Game/Lobby/BP_LobbyGameState.SelectedNewColor_OnServer` _asbp_lobby_game_state (`/Game/Blueprints/Game/Lobby/Character/BP_LobbyCharacter.CharacterColor` (`/Game/Blueprints/Game/Lobby/BP_LobbyPlayerController.LobbyCharacter` Controller)) Material)
  (`/Game/Blueprints/Game/Lobby/BP_LobbyPlayerController.UpdateLobbyCharColor_OnServer` Controller Material))

(fn `SetRandomCharacterColor`
  (params (Controller :type "/Game/Blueprints/Game/Lobby/BP_LobbyPlayerController Object Reference"))
  (locals (Color :type "MaterialInstance Object Reference"))
  (bind _asbp_lobby_game_state (cast `/Game/Blueprints/Game/Lobby/BP_LobbyGameState` (`GameplayStatics.GetGameState`)))
  (bind _availablecolorsout (`/Game/Blueprints/Game/Lobby/BP_LobbyGameState.GetAvailableColors` _asbp_lobby_game_state))
  (bind _output_get (set `local.Color` (`|GetArrayItem` _availablecolorsout (`KismetMathLibrary.RandomInteger` (- (`KismetArrayLibrary.Array_Length` _availablecolorsout) 1)))))
  (`/Game/Blueprints/Game/Lobby/BP_LobbyGameState.AddOrRemoveColorToBlock_OnServer` _asbp_lobby_game_state _output_get false)
  (`/Game/Blueprints/Game/Lobby/BP_LobbyPlayerController.UpdateLobbyCharColor_OnServer` Controller (`local.Color`)))

(fn `UserConstructionScript`)