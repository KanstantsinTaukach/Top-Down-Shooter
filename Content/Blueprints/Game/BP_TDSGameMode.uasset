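; Game mode for a multiplayer top-down zombie shooter that handles player joining, phase-based respawning and enemy spawning.
; A looping timer asks BP_GameState for the current phase, score budget and wave index, then finds the matching BP_EnemySpawner.
; Random enemy types up to that wave spawn inside the spawner's box while spawned kill score is under budget.
; Joining players get GameInstance colors, and enemy deaths feed points to the game state.
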(event `self.ReceiveBeginPlay`
  (`KismetSystemLibrary.K2_SetTimer` null "TrySpawnEnemy" 0.2 true))

(event `self.HandleStartingNewPlayer`
  (params (NewPlayer :type "PlayerController Object Reference"))
  (`parent.HandleStartingNewPlayer` NewPlayer)
  (`KismetArrayLibrary.Array_Add` (`self.Controllers`) NewPlayer)
  (bind _asbp_tdsgame_instance (cast `/Game/Blueprints/Game/BP_TDSGameInstance` (`GameplayStatics.GetGameInstance`)))
  (bind _asbp_tdscharacter (cast `/Game/Blueprints/Character/BP_TDSCharacter` (`Controller.K2_GetPawn` NewPlayer)))
  (`/Game/Blueprints/Character/BP_TDSCharacter.SetCharacterMaterial_OnServer` _asbp_tdscharacter (`BlueprintMapLibrary.Map_Find` (`/Game/Blueprints/Game/BP_TDSGameInstance.ColorForPlayers` _asbp_tdsgame_instance) (`KismetStringLibrary.Conv_IntToString` (`PlayerState.PlayerId` (`Controller.PlayerState` NewPlayer))))))

(event `self.K2_OnLogout`
  (params (ExitingController :type "Controller Object Reference"))
  (`KismetArrayLibrary.Array_RemoveItem` (`self.Controllers`) ExitingController))

(fn `ChoosePlayerStart`
  (params (Player :type "Controller Object Reference"))
  (returns (ReturnValue :type "Actor Object Reference"))
  (return (`self.K2_FindPlayerStart` Player "Phase1")))

(fn `EnemyDead`
  (params (Points :type Integer))
  (set `self.NumberOfEnemies` (- (`self.NumberOfEnemies`) 1))
  (bind _asbp_game_state (cast `/Game/Blueprints/Game/BP_GameState` (`GameplayStatics.GetGameState`)))
  (`/Game/Blueprints/Game/BP_GameState.AddPoints` _asbp_game_state Points))

(fn `GetCurrentEnemySpawner`
  (params (NumberOfSpawnedEnemies :type Integer))
  (bind _asbp_game_state (cast `/Game/Blueprints/Game/BP_GameState` (`GameplayStatics.GetGameState`)))
  (bind (_currentphase _currentphasescore _currentenemywaveindex) (`/Game/Blueprints/Game/BP_GameState.GetEnemyPhase` _asbp_game_state NumberOfSpawnedEnemies))
  (bind _outactors (`GameplayStatics.GetAllActorsOfClass` "/Game/Blueprints/InteractionEnvironment/EnemySpawner/BP_EnemySpawner.BP_EnemySpawner_C"))
  (bind _output_get (set `self.EnemySpawners` _outactors))
  (for _array_element _output_get
    (if (`|EnumEquality` (`/Game/Blueprints/InteractionEnvironment/EnemySpawner/BP_EnemySpawner.Phase` _array_element) _currentphase)
      (set `self.CurrentSpawner` _array_element)
      (break)))
  (set `self.Current Phase Score` _currentphasescore)
  (set `self.EnemyWaveIndex` _currentenemywaveindex))

(fn `TrySpawnEnemy`
  (bind _currentspawner (`self.CurrentSpawner`))
  (`self.GetCurrentEnemySpawner` (`self.NumberOfEnemies`))
  (if (< (`self.CurrentSpawnerScore`) (`self.Current Phase Score`))
    (bind _returnvalue (`|SpawnActorFromClass` (select `int` (`KismetMathLibrary.RandomIntegerInRange` 0 (`self.EnemyWaveIndex`)) :`0` "/Game/Blueprints/AI/Characters/Zombiegirl/BP_TDSAICharacter_ZombieGirl.BP_TDSAICharacter_ZombieGirl_C" :`1` "/Game/Blueprints/AI/Characters/Warzombie/BP_TDSAICharacter_WarZombie.BP_TDSAICharacter_WarZombie_C" :`2` "/Game/Blueprints/AI/Characters/Parasite/BP_TDSAICharacter_Parasite.BP_TDSAICharacter_Parasite_C" :`3` "/Game/Blueprints/AI/Boss/BP_TDSAICharacter_Boss.BP_TDSAICharacter_Boss_C" :!type "Actor Class Reference") (`KismetMathLibrary.Conv_VectorToTransform` (`KismetMathLibrary.RandomPointInBoundingBox` (`self.K2_GetActorLocation` _currentspawner) (`BoxComponent.BoxExtent` (`/Game/Blueprints/InteractionEnvironment/EnemySpawner/BP_EnemySpawner.Box` _currentspawner)))) "Undefined" "OverrideRootScale" null null))
    (`/Engine/EditorBlueprintResources/StandardMacros.IsValid` _returnvalue
      (:`Is Valid`
        (set `self.CurrentSpawnerScore` (+ (`self.CurrentSpawnerScore`) (`/Game/Blueprints/Components/BP_KillScoreComponent.Score` (`self.GetComponentByClass` _returnvalue "/Game/Blueprints/Components/BP_KillScoreComponent.BP_KillScoreComponent_C"))))
        (set `self.NumberOfEnemies` (+ (`self.NumberOfEnemies`) 1))))))

(fn `TryToRespawnPlayer`
  (returns (bIsSuccess :type Boolean))
  (bind _asbp_game_state (cast `/Game/Blueprints/Game/BP_GameState` (`GameplayStatics.GetGameState`)))
  (bind (_bcanplayerrespawn _currentphase) (`/Game/Blueprints/Game/BP_GameState.CanPlayerRespawn` _asbp_game_state))
  (if _bcanplayerrespawn
    (`self.RestartPlayerAtPlayerStart` (`GameplayStatics.GetPlayerController` 0) (`self.K2_FindPlayerStart` null (`|GetEnumeratorNameAsString` _currentphase)))
    (return _bcanplayerrespawn)
    (else
      (return _bcanplayerrespawn))))

(fn `UserConstructionScript`)