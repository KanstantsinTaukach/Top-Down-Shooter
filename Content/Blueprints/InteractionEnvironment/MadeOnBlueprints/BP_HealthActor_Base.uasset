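; Base actor for damageable, destructible environment objects with a TDSHealth component.
; Any damage is printed and subtracted from health; each hit reported by the component spawns a randomly offset BP_DisplayDamageActor showing health and damage.
; Radial damage from a TDS_ProjectileDefault also applies that projectile's effect according to the mesh material's physical surface type.
; On death the actor destroys itself with a collapse sound and explosion particles.
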(event `self.TDSHealth.OnTakeDamage`
  (params (Health :type "Float (single-precision)") (Damage :type "Float (single-precision)"))
  (bind _returnvalue (`|SpawnActorFromClass` "/Game/Blueprints/InteractionEnvironment/MadeOnBlueprints/BP_DisplayDamageActor.BP_DisplayDamageActor_C" (`KismetMathLibrary.Conv_VectorToTransform` (+ (`self.K2_GetActorLocation`) (+ (`KismetMathLibrary.MakeVector` (`KismetMathLibrary.RandomFloatInRange` -20.0 20.0) (`KismetMathLibrary.RandomFloatInRange` -20.0 20.0)) (`self.LocalPointSpawnerHealthNumbers`)))) "AlwaysSpawn" "OverrideRootScale" null null))
  (`/Game/Blueprints/InteractionEnvironment/MadeOnBlueprints/BP_DisplayDamageActor.InitActor` _returnvalue Health Damage))

(event `self.TDSHealth.OnDeath`
  (`self.DestroyActor`))

(event `self.ReceiveAnyDamage`
  (params (Damage :type "Float (single-precision)") (DamageType :type "DamageType Object Reference") (InstigatedBy :type "Controller Object Reference") (DamageCauser :type "Actor Object Reference"))
  (`KismetSystemLibrary.PrintString` (`KismetStringLibrary.Conv_DoubleToString` Damage))
  (`TDSHealthComponent.RemoveFromCurrentHealth` (`self.TDSHealth`) Damage))

(event `self.ReceivePointDamage`
  (params (Damage :type "Float (single-precision)") (DamageType :type "DamageType Object Reference") (HitLocation :type "Vector Structure") (HitNormal :type "Vector Structure") (HitComponent :type "PrimitiveComponent Object Reference") (BoneName :type Name) (ShotFromDirection :type "Vector Structure") (InstigatedBy :type "Controller Object Reference") (DamageCauser :type "Actor Object Reference") (HitInfo :type "HitResult Structure (by ref)")))

(event `self.ReceiveRadialDamage`
  (params (DamageReceived :type "Float (single-precision)") (DamageType :type "DamageType Object Reference") (Origin :type "Vector Structure") (HitInfo :type "HitResult Structure (by ref)") (InstigatedBy :type "Controller Object Reference") (DamageCauser :type "Actor Object Reference"))
  (bind _astds_projectile_default (cast `TDS_ProjectileDefault` DamageCauser))
  (`Types.AddEffectBySurfaceType` self (`.Effect` (break `ProjectileInfo` (`TDS_ProjectileDefault.ProjectileSettings` _astds_projectile_default))) (`PhysicalMaterial.SurfaceType` (`MaterialInterface.GetPhysicalMaterial` (`PrimitiveComponent.GetMaterial` (`self.StaticMesh`) 0)))))

(fn `DestroyActor`
  (bind _returnvalue (`self.K2_GetActorLocation`))
  (`self.K2_DestroyActor`)
  (`GameplayStatics.SpawnSoundAtLocation` "/Game/Sounds/Collapse_Cue.Collapse_Cue" _returnvalue (struct) 1.0 1.0 0.0 null null)
  (`GameplayStatics.SpawnEmitterAtLocation` "/Game/Items/MilitaryWeapons/FX/P_Grenade_Explosion_01.P_Grenade_Explosion_01" _returnvalue))

(fn `UserConstructionScript`)