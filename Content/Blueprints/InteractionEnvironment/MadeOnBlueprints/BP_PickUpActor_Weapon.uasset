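; Weapon pickup actor that tries to add its weapon to the inventory of an overlapping character.
; InitActor takes the weapon slot data from the drop item info before running the parent initialization.
; On character overlap, it passes that slot to the inventory's TryGetWeaponToInventory and calls PickUpSuccess if accepted.
; The failure branch only casts the inventory owner to BP_Character, with no further action.
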(event `self.OnCharacterOverlap`
  (params (Inventory :type "TDSInventoryComponent Object Reference"))
  (`parent.OnCharacterOverlap` Inventory)
  (bind _returnvalue (`TDSInventoryComponent.TryGetWeaponToInventory` Inventory (`self.WeaponSlot`)))
  (if _returnvalue
    (`self.PickUpSuccess`)
    (else
      (cast `/Game/Blueprints/Character/BP_Character` (`ActorComponent.GetOwner` Inventory)))))

(fn `InitActor`
  (params (DropItemInfo :type "DropItem Structure"))
  (set `self.WeaponSlot` (`.WeaponSlotInfo` (break `DropItem` DropItemInfo)))
  (`parent.InitActor` DropItemInfo))

(fn `UserConstructionScript`
  (`parent.UserConstructionScript`))