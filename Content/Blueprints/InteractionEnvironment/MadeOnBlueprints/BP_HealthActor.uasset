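; BP_HealthActor is a damageable environment actor that shows floating damage feedback and explodes on death.
; AnyDamage feeds the TDSHealth component, while point and radial damage events only print their values.
; Each health change spawns a BP_DisplayDamageActor at a randomly jittered offset, initialized with current health and damage taken.
; On death, the DestroyActor function removes the actor and spawns a collapse sound and grenade explosion effect.
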(event `self.ReceiveBeginPlay`
  (bind _tdshealth (`self.TDSHealth`))
  (add `TDSHealthComponent.OnHealthChanged` _tdshealth (delegate `OnHealthChanged_Event`))
  (add `TDSHealthComponent.OnDeath` _tdshealth (delegate `OnDeath_Event`)))

(event `OnDeath_Event`
  (`self.DestroyActor`))

(event `OnHealthChanged_Event`
  (params (Health :type "Float (double-precision)") (Damage :type "Float (double-precision)"))
  (bind _returnvalue (`|SpawnActorFromClass` "/Game/Blueprints/InteractionEnvironment/MadeOnBlueprints/BP_DisplayDamageActor.BP_DisplayDamageActor_C" (`KismetMathLibrary.Conv_VectorToTransform` (+ (`self.K2_GetActorLocation`) (+ (`KismetMathLibrary.MakeVector` (`KismetMathLibrary.RandomFloatInRange` -20.0 20.0) (`KismetMathLibrary.RandomFloatInRange` -20.0 20.0)) (`self.LocalPointSpawnerHealthNumbers`)))) "AlwaysSpawn" "OverrideRootScale" null null))
  (`/Game/Blueprints/InteractionEnvironment/MadeOnBlueprints/BP_DisplayDamageActor.InitActor` _returnvalue Health Damage))

(event `self.ReceiveAnyDamage`
  (params (Damage :type "Float (single-precision)") (DamageType :type "DamageType Object Reference") (InstigatedBy :type "Controller Object Reference") (DamageCauser :type "Actor Object Reference"))
  (`KismetSystemLibrary.PrintString` (`KismetStringLibrary.Conv_DoubleToString` Damage))
  (`TDSHealthComponent.ReceiveDamage` (`self.TDSHealth`) Damage))

(event `self.ReceivePointDamage`
  (params (Damage :type "Float (single-precision)") (DamageType :type "DamageType Object Reference") (HitLocation :type "Vector Structure") (HitNormal :type "Vector Structure") (HitComponent :type "PrimitiveComponent Object Reference") (BoneName :type Name) (ShotFromDirection :type "Vector Structure") (InstigatedBy :type "Controller Object Reference") (DamageCauser :type "Actor Object Reference") (HitInfo :type "HitResult Structure (by ref)"))
  (`KismetSystemLibrary.PrintString` (`KismetStringLibrary.Conv_DoubleToString` Damage) true true (struct :`G` 1.0 :`B` 0.216083 :`A` 1.0)))

(event `self.ReceiveRadialDamage`
  (params (DamageReceived :type "Float (single-precision)") (DamageType :type "DamageType Object Reference") (Origin :type "Vector Structure") (HitInfo :type "HitResult Structure (by ref)") (InstigatedBy :type "Controller Object Reference") (DamageCauser :type "Actor Object Reference"))
  (`KismetSystemLibrary.PrintString` (`KismetStringLibrary.Conv_DoubleToString` DamageReceived) true true (struct :`R` 1.0 :`G` 0.489736 :`A` 1.0)))

(fn `DestroyActor`
  (bind _returnvalue (`self.K2_GetActorLocation`))
  (`self.K2_DestroyActor`)
  (`GameplayStatics.SpawnSoundAtLocation` "/Game/Sounds/Collapse_Cue.Collapse_Cue" _returnvalue (struct) 1.0 1.0 0.0 null null)
  (`GameplayStatics.SpawnEmitterAtLocation` "/Game/Items/MilitaryWeapons/FX/P_Grenade_Explosion_01.P_Grenade_Explosion_01" _returnvalue))

(fn `UserConstructionScript`)