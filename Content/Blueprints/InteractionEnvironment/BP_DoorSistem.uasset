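; BP_DoorSistem is an automatic door that moves along its Z axis when a BP_Character walks into its trigger volumes.
; Overlapping EnterTrigger calls Opening and overlapping ExitTrigger calls Closing, with the IsDoorOpen flag preventing repeated runs.
; A single timeline plays forward to open and reverses to close, its curve mapped to the Z variable to set the door's relative height.
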(event `self.EnterTrigger.OnComponentBeginOverlap`
  (params (OverlappedComponent :type "PrimitiveComponent Object Reference") (OtherActor :type "Actor Object Reference") (OtherComp :type "PrimitiveComponent Object Reference") (OtherBodyIndex :type Integer) (bFromSweep :type Boolean) (SweepResult :type "HitResult Structure (by ref)"))
  (cast `/Game/Blueprints/Character/BP_Character` OtherActor)
  (`self.Opening`))

(event `self.ExitTrigger.OnComponentBeginOverlap`
  (params (OverlappedComponent :type "PrimitiveComponent Object Reference") (OtherActor :type "Actor Object Reference") (OtherComp :type "PrimitiveComponent Object Reference") (OtherBodyIndex :type Integer) (bFromSweep :type Boolean) (SweepResult :type "HitResult Structure (by ref)"))
  (cast `/Game/Blueprints/Character/BP_Character` OtherActor)
  (`self.Closing`))

(event `Opening`
  (if (not (`self.bIsDoorOpen`))
    (set `self.bIsDoorOpen` true)
    (bind (_direction _zoffset) (`Timeline|OpenDoorTimeline` :!label _label)
      (:`Update`
        (`SceneComponent.K2_SetRelativeLocation` (`self.Door`) (`KismetMathLibrary.MakeVector` 0.0 0.0 (`KismetMathLibrary.MapRangeClamped` _zoffset 0.0 1.0 0.0 (`self.Z`))) false false)))))

(event `Closing`
  (if (`self.bIsDoorOpen`)
    (set `self.bIsDoorOpen` false)
    (goto _label :!via `Reverse`)))

(fn `UserConstructionScript`)