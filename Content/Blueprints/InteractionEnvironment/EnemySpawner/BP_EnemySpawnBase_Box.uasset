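; Box-shaped enemy spawner that continuously creates parasite AI characters within its volume.
; BeginPlay starts a looping one-second timer that spawns one BP_TDSAICharacter_Parasite at a random point inside the Box component's extent around the actor's location.
; Spawns shift to avoid collisions or are skipped if no free spot is found, and the graph sets no limit on the enemy count.
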(event `self.ReceiveBeginPlay`
  (`parent.ReceiveBeginPlay`)
  (`KismetSystemLibrary.K2_SetTimerDelegate` (delegate `CustomEvent_0`) 1.0 true))

(event `CustomEvent_0`
  (`|SpawnActorFromClass` "/Game/Blueprints/AI/BP_TDSAICharacter_Parasite.BP_TDSAICharacter_Parasite_C" (`KismetMathLibrary.Conv_VectorToTransform` (`KismetMathLibrary.RandomPointInBoundingBox` (`self.K2_GetActorLocation`) (`BoxComponent.BoxExtent` (`self.Box`)))) "AdjustIfPossibleButDontSpawnIfColliding" "OverrideRootScale" null null))

(fn `UserConstructionScript`
  (`parent.UserConstructionScript`))