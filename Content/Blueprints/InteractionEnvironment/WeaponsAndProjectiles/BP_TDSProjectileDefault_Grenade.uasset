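; Grenade projectile Blueprint for the TDS weapons set that blinks a point light while active.
; BeginPlay starts a looping Flash timer at MaxFlashTime, and each call applies, then inverts, the light's visibility flag.
; Flash also counts FlashTime down, but never resets the timer, so the blink interval stays constant.
; No movement or explosion logic is defined in these graphs.
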(event `self.ReceiveBeginPlay`
  (bind _output_get (set `self.FlashTime` (`self.MaxFlashTime`)))
  (`KismetSystemLibrary.K2_SetTimer` self "Flash" _output_get true))

(fn `Flash`
  (bind _flashtime (`self.FlashTime`))
  (`SceneComponent.SetVisibility` (`self.PointLight`) (`self.IsEnable`) false)
  (if (> _flashtime 0.0)
    (set `self.FlashTime` (- _flashtime 0.1))
    (else
      (set `self.FlashTime` 0.1)))
  (if (`self.IsEnable`)
    (set `self.IsEnable` false)
    (else
      (set `self.IsEnable` true))))

(fn `UserConstructionScript`)