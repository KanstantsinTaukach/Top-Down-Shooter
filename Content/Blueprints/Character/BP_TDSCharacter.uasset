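; Player character Blueprint for a top-down shooter, layering presentation and UI over health, inventory and weapon events.
; Damage drives blood material, random decals and sounds, while shield events swap materials on a shell mesh that follows the body's pose.
; Tick feeds a sprint Niagara trail and slides the local camera boom toward the cursor while aiming.
; Weapon events update animation and HUD; pause and death handle menus, respawn or game over.
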(event `self.CharacterHealthComponent.OnTakeDamage`
  (params (Health :type "Float (single-precision)") (Damage :type "Float (single-precision)"))
  ;[1 1 1] BloodFX
  (`|ExecutionSequence`
    (:`then_0`
      (`self.SpawnBloodOnCharacter` Health)
      (`GameplayStatics.PlaySoundAtLocation` "/Game/Sounds/PlayerTakesDamage_Cue.PlayerTakesDamage_Cue" (`SceneComponent.K2_GetComponentLocation` (`self.Mesh`)) (struct) 1.0 1.0 0.0 null null null))
    (:`then_1`
      (`self.SpawnBloodDecal` Damage))))

(event `self.CharacterHealthComponent.OnHealthChanged`
  (params (Health :type "Float (single-precision)") (HealthValue :type "Float (single-precision)"))
  ;[1 1 1] BloodFX
  (`self.SpawnBloodOnCharacter` Health))

(event `self.ReceiveTick`
  (params (DeltaSeconds :type "Float (single-precision)"))
  ;[1 0.02953 0] Camera Slide TODO: SprintFX
  (`self.SetNiagaraTrail`)
  (if (`self.IsLocallyControlled`)
    (`self.CameraSlideToCursor` DeltaSeconds)))

(event `self.CharacterHealthComponent.OnShieldTakeDamage`
  (params (Shield :type "Float (single-precision)") (Damage :type "Float (single-precision)"))
  (bind _sk_shellmannequin (`self.SK_ShellMannequin`))
  ;[1 1 1] ShieldFx
  (`PrimitiveComponent.SetMaterial` (`self.SK_ShellMannequin`) 0 "/Game/Fx_Effects/Shield/MI_EnergyDamage.MI_EnergyDamage")
  (`GameplayStatics.PlaySoundAtLocation` "/Game/Sounds/ShieldHits_Cue.ShieldHits_Cue" (`SceneComponent.K2_GetComponentLocation` (`self.Mesh`)) (struct) 1.0 1.0 0.0 null null null)
  (`KismetSystemLibrary.Delay` 0.5)
  (if (> Shield 0.0)
    (`PrimitiveComponent.SetMaterial` _sk_shellmannequin 0 (`self.MeshMaterial`))
    (else
      (`PrimitiveComponent.SetMaterial` _sk_shellmannequin 0 "/Game/Fx_Effects/Shield/MI_EnergyEmpty.MI_EnergyEmpty"))))

(event `self.CharacterHealthComponent.OnShieldChanged`
  (params (Shield :type "Float (single-precision)") (ChangeValue :type "Float (single-precision)"))
  ;[1 1 1] ShieldFx
  (`self.ShieldCharging` Shield ChangeValue))

(event `self.ReceiveBeginPlay`
  (`|ExecutionSequence`
    (:`then_0`
      (bind _asabp_third_person (cast `/Game/Blueprints/Character/Mannequin/Animations/ABP_ThirdPerson` (`SkeletalMeshComponent.GetAnimInstance` (`self.Mesh`))))
      (set `self.CharAnimInstance` _asabp_third_person)
      (bind _asbp_tdsplayer_controller (cast `/Game/Blueprints/Game/BP_TDSPlayerController` (`self.GetController`)))
      (bind _asbp_tdscharacter (cast `/Game/Blueprints/Character/BP_TDSCharacter` (`Controller.K2_GetPawn` _asbp_tdsplayer_controller)))
      (bind _output_get (set `self.TDSCharacterRef` _asbp_tdscharacter))
      (bind _asbp_tdshud (cast `/Game/Blueprints/UI/BP_TDSHUD` (`PlayerController.GetHUD` _asbp_tdsplayer_controller)))
      (bind _aswbp_gameplay (cast `/Game/Blueprints/UI/WBP_Gameplay` (`TDS_HUD.GetGameplayWidget` _asbp_tdshud)))
      (`/Game/Blueprints/UI/Inventory/WBP_InventoryStats.InitInventoryStatsWidget` (`/Game/Blueprints/UI/WBP_Gameplay.WBP_InventoryStats` _aswbp_gameplay) _output_get))
    (:`then_1`
      (if (`|EnumEquality` (`self.GetLocalRole`) "ROLE_SimulatedProxy")
        (`PrimitiveComponent.SetMaterial` (`self.SK_ShellMannequin`) 0 (`self.MeshMaterial`))))))

(event `SetCharacterMaterial_OnServer`
  (params (MeshMaterial :type "MaterialInterface Object Reference"))
  (`self.SetCharacterMaterical_Multicast` MeshMaterial))

(event `SetCharacterMaterical_Multicast`
  (params (MeshMaterial :type "MaterialInterface Object Reference"))
  (bind _keys (`BlueprintMapLibrary.Map_Keys` (`self.StartMaterials`)))
  (for (_array_element _array_index) _keys
    (if (== _array_element MeshMaterial)
      (bind _values (`BlueprintMapLibrary.Map_Values` (`self.StartMaterials`)))
      (bind _output_get (set `self.MeshMaterial` (`|GetArrayItem` _values _array_index)))
      (`PrimitiveComponent.SetMaterial` (`self.SK_ShellMannequin`) 0 _output_get))))

(event `self.WeaponReloadEnd_BP`
  (params (bIsSuccess :type Boolean))
  ;[1 1 1] FireAndReload (Animation and UI)
  (`/Game/Blueprints/Character/Mannequin/Animations/ABP_ThirdPerson.ReloadEnd` (`self.CharAnimInstance`) bIsSuccess)
  (bind _aswbp_gameplay (`self.Get_WBPGameplayWidget`))
  (`/Engine/EditorBlueprintResources/StandardMacros.IsValid` _aswbp_gameplay
    (:`Is Valid`
      (`/Game/Blueprints/UI/Inventory/WBP_InventoryStats.WeaponReloadEnd` (`/Game/Blueprints/UI/WBP_Gameplay.WBP_InventoryStats` _aswbp_gameplay) (`self.GetCurrentWeaponIndex`) bIsSuccess))))

(event `self.WeaponReloadStart_BP`
  (params (AnimMontage :type "AnimMontage Object Reference"))
  ;[1 1 1] FireAndReload (Animation and UI)
  (`/Game/Blueprints/Character/Mannequin/Animations/ABP_ThirdPerson.Reload` (`self.CharAnimInstance`) AnimMontage)
  (bind _aswbp_gameplay (`self.Get_WBPGameplayWidget`))
  (`/Engine/EditorBlueprintResources/StandardMacros.IsValid` _aswbp_gameplay
    (:`Is Valid`
      (`/Game/Blueprints/UI/Inventory/WBP_InventoryStats.WeaponReloadStart` (`/Game/Blueprints/UI/WBP_Gameplay.WBP_InventoryStats` _aswbp_gameplay) (`self.GetCurrentWeaponIndex`)))))

(event `self.InventoryComponent.OnSwitchWeapon`
  (params (WeaponName :type Name) (AdditionalWeaponInfo :type "AdditionalWeaponInfo Structure") (NewCurrentWeaponIndex :type Integer))
  ;[1 1 1] FireAndReload (Animation and UI)
  (bind _aswbp_gameplay (`self.Get_WBPGameplayWidget`))
  (`/Engine/EditorBlueprintResources/StandardMacros.IsValid` _aswbp_gameplay
    (:`Is Valid`
      (bind _aswbp_weapon_slot (cast `/Game/Blueprints/UI/Inventory/WBP_WeaponSlot` (`PanelWidget.GetChildAt` (`/Game/Blueprints/UI/Inventory/WBP_InventoryStats.WeaponSlots` (`/Game/Blueprints/UI/WBP_Gameplay.WBP_InventoryStats` _aswbp_gameplay)) NewCurrentWeaponIndex)))
      (`/Game/Blueprints/UI/Inventory/WBP_WeaponSlot.UpdateInfo` _aswbp_weapon_slot WeaponName (`.Round` (break `AdditionalWeaponInfo` AdditionalWeaponInfo))))))

(event `self.WeaponFire_BP`
  (params (AnimMontage :type "AnimMontage Object Reference"))
  ;[1 1 1] FireAndReload (Animation and UI)
  (`/Game/Blueprints/Character/Mannequin/Animations/ABP_ThirdPerson.Fire` (`self.CharAnimInstance`) AnimMontage))

(event `InputAction|PauseGame` :paused true
  (params (Key :type "Key Structure"))
  (bind _returnvalue (`GameplayStatics.GetPlayerController` 0))
  (bind _pausemenureference (`self.PauseMenuReference`))
  ;[1 1 1] Pause/Unpause game
  (:`Pressed`
    (`/Engine/EditorBlueprintResources/StandardMacros.IsValid` (`self.PauseMenuReference`)
      (:`Is Valid`
        _)
      (:`Is Not Valid`
        (bind _returnvalue_2 (`|CreateWidget` "/Game/Blueprints/UI/Menu/WBP_PauseMenu.WBP_PauseMenu_C"))
        (set `self.PauseMenuReference` _returnvalue_2)))
    (if (`GameplayStatics.IsGamePaused`)
      (`Widget.RemoveFromParent` _pausemenureference)
      (`GameplayStatics.SetGamePaused` false)
      (set `PlayerController.bShowMouseCursor` false _returnvalue)
      (`WidgetBlueprintLibrary.SetInputMode_GameOnly` _returnvalue)
      (else
        (`UserWidget.AddToViewport` _pausemenureference 0)
        (`GameplayStatics.SetGamePaused` true)
        (set `PlayerController.bShowMouseCursor` true _returnvalue)
        (`WidgetBlueprintLibrary.SetInputMode_GameAndUIEx` _returnvalue (`self.PauseMenuReference`) "LockInFullscreen" false)))))

(event `self.OnCharacterDeath_BP`
  ;[1 1 1] GameOver
  (bind _returnvalue (`self.GetCurrentWeapon`))
  (`self.SetLifeSpan` _returnvalue 10.0)
  (`self.SetLifeSpan` 10.0)
  (`self.TryToContinueGame`))

(fn `CameraSlideToCursor`
  (params (InputPin :type "Float (double-precision)"))
  (bind _cameraboom (`self.CameraBoom`))
  (bind _returnvalue (`SceneComponent.K2_GetComponentLocation` (`self.CapsuleComponent`)))
  (bind (_returnvalue_x _returnvalue_y _returnvalue_z) (`KismetMathLibrary.BreakVector` (`SceneComponent.K2_GetComponentLocation` (`self.CameraBoom`))))
  (bind _returnvalue_2 (`self.GetCursorToWorld`))
  (set `self.ClampedCameraHeight` (`KismetMathLibrary.MapRangeClamped` (`SpringArmComponent.TargetArmLength` (`self.CameraBoom`)) (`self.CameraHeightMin`) (`self.CameraHeightMax`) 0.5 1.0))
  (bind _returnvalue_3 (`SceneComponent.K2_GetComponentLocation` _returnvalue_2))
  (set `self.DistanceCameraBoomChar` (`KismetMathLibrary.VSizeXY` (- _returnvalue _returnvalue_3)))
  (if (`|EnumEquality` (`self.MovementState`) "Aim_State")
    (if (> (`self.DistanceCameraBoomChar`) (* (`self.ClampedCameraHeight`) (`self.FMinClampDistanceLogicMouseCursorStart`)))
      (if (not (> (`KismetMathLibrary.VSize2D` (`KismetMathLibrary.Conv_VectorToVector2D` (- (`SceneComponent.K2_GetComponentLocation` (`self.CameraBoom`)) _returnvalue))) (* (`self.ClampedCameraHeight`) (`self.FMaxClampDistanceLogicMouseCursorStart`))))
        (bind (_x _y) (`KismetMathLibrary.BreakVector2D` (* (`KismetMathLibrary.Normal2D` (`KismetMathLibrary.Conv_VectorToVector2D` (`KismetMathLibrary.GetForwardVector` (`KismetMathLibrary.FindLookAtRotation` _returnvalue _returnvalue_3)))) (`self.FSpeedChangeLocationCameraToCursor`))))
        (`SceneComponent.K2_SetWorldLocation` (`self.CameraBoom`) (`KismetMathLibrary.MakeVector` (+ _x _returnvalue_x) (+ _y _returnvalue_y) _returnvalue_z) false false))
      (else
        (`SceneComponent.K2_SetWorldLocation` _cameraboom (`KismetMathLibrary.VInterpTo` (`SceneComponent.K2_GetComponentLocation` _cameraboom) (`SceneComponent.K2_GetComponentLocation` (`self.CapsuleComponent`)) InputPin (`self.FSpeedReturnCameraDefaultPosition`)) false false :!label _label)))
    (else
      (goto _label))))

(fn `CheckCanAttack`
  (returns (CanAttack :type Boolean))
  (return false))

(fn `CheckCanMove`
  (returns (CanMove :type Boolean))
  (return false))

(fn `Get_WBPGameplayWidget`
  (returns (`AsWBP Gameplay` :type "/Game/Blueprints/UI/WBP_Gameplay Object Reference"))
  (bind _asbp_tdsplayer_controller (cast `/Game/Blueprints/Game/BP_TDSPlayerController` (`self.GetController`)))
  (bind _asbp_tdshud (cast `/Game/Blueprints/UI/BP_TDSHUD` (`PlayerController.GetHUD` _asbp_tdsplayer_controller)))
  (bind _aswbp_gameplay (cast `/Game/Blueprints/UI/WBP_Gameplay` (`TDS_HUD.GetGameplayWidget` _asbp_tdshud)))
  (return _aswbp_gameplay))

(fn `SetNiagaraTrail`
  (if (`self.IsSprinting` self)
    (`NiagaraComponent.SetVariableFloat` (`self.NS_Trail`) "Sprint" (`KismetMathLibrary.VSize` (`MovementComponent.Velocity` (`self.CharacterMovement`))))
    (else
      (`NiagaraComponent.SetVariableFloat` (`self.NS_Trail`) "Sprint" 0.0))))

(fn `ShieldCharging`
  (params (CurrentShield :type "Float (double-precision)") (ChangeValue :type "Float (double-precision)"))
  (bind _returnvalue (`SceneComponent.K2_GetComponentLocation` (`self.Mesh`)))
  (`GameplayStatics.PlaySoundAtLocation` "/Game/Sounds/ShieldCharge_Cue1.ShieldCharge_Cue1" _returnvalue (struct) 0.1 1.0 0.0 null null null)
  (`AISense_Hearing.ReportNoiseEvent` _returnvalue 1.0 self)
  (`PrimitiveComponent.SetMaterial` (`self.SK_ShellMannequin`) 0 "/Game/Fx_Effects/Shield/MI_EnergyCharge.MI_EnergyCharge")
  (if (== CurrentShield 100.0)
    (`PrimitiveComponent.SetMaterial` (`self.SK_ShellMannequin`) 0 "/Game/Fx_Effects/Shield/MI_EnergyFull.MI_EnergyFull")))

(fn `SpawnBloodDecal`
  (params (Damage :type "Float (double-precision)"))
  (if (> Damage 0.0)
    (if (> (`KismetMathLibrary.RandomFloat`) 0.3)
      (`GameplayStatics.SpawnDecalAtLocation` (select `int` (`KismetMathLibrary.RandomIntegerInRange` 0 1) :`0` "/Game/Blueprints/Decals/BloodSpatter/M_Decal_BloodSpatter.M_Decal_BloodSpatter" :`1` "/Game/Blueprints/Decals/BloodSpatter2/M_Decal_BloodSpatter2.M_Decal_BloodSpatter2" :`2` "/Game/Blueprints/Decals/BloodStain/M_Decal_BloodStain.M_Decal_BloodStain" :!type "MaterialInterface Object Reference") (30.0 60.0 60.0) (- (`self.K2_GetActorLocation`) (`KismetMathLibrary.MakeVector` (`KismetMathLibrary.RandomFloatInRange` -30.0 30.0) (`KismetMathLibrary.RandomFloatInRange` -30.0 30.0) 115.0)) (struct :`Pitch` -90.0) 10.0))))

(fn `SpawnBloodOnCharacter`
  (params (Health :type "Float (double-precision)"))
  (bind _returnvalue (`KismetMathLibrary.MapRangeClamped` Health 50.0 100.0 1.0))
  (bind _returnvalue_2 (`PrimitiveComponent.GetMaterial` (`self.Mesh`) 0))
  (bind _asmaterial_instance_dynamic (cast `MaterialInstanceDynamic` _returnvalue_2)
    (:`then`
      (`MaterialInstanceDynamic.SetScalarParameterValue` _asmaterial_instance_dynamic "Blood" _returnvalue))
    (:`CastFailed`
      (bind _returnvalue_3 (`PrimitiveComponent.CreateDynamicMaterialInstance` (`self.Mesh`) 0 _returnvalue_2 "BloodDynamic"))
      (`MaterialInstanceDynamic.SetScalarParameterValue` _returnvalue_3 "Blood" _returnvalue)
      (`PrimitiveComponent.SetMaterial` (`self.Mesh`) 0 _returnvalue_3))))

(fn `TryToContinueGame`
  (bind _returnvalue (`GameplayStatics.GetPlayerController` 0))
  (bind _endgamemenureference (`self.EndGameMenuReference`))
  (bind _asbp_tdsgame_mode (cast `/Game/Blueprints/Game/BP_TDSGameMode` (`GameplayStatics.GetGameMode`)))
  (bind _bissuccess (`/Game/Blueprints/Game/BP_TDSGameMode.TryToRespawnPlayer` _asbp_tdsgame_mode))
  (if _bissuccess
    (bind _asbp_tdsplayer_controller (cast `/Game/Blueprints/Game/BP_TDSPlayerController` (`GameplayStatics.GetPlayerController` 0)))
    (bind _asbp_tdshud (cast `/Game/Blueprints/UI/BP_TDSHUD` (`PlayerController.GetHUD` _asbp_tdsplayer_controller)))
    (bind _aswbp_gameplay (cast `/Game/Blueprints/UI/WBP_Gameplay` (`TDS_HUD.GetGameplayWidget` _asbp_tdshud)))
    (`/Game/Blueprints/UI/Inventory/WBP_InventoryStats.UnbindAllEvents` (`/Game/Blueprints/UI/WBP_Gameplay.WBP_InventoryStats` _aswbp_gameplay) (`self.TDSCharacterRef`))
    (bind _asbp_tdscharacter (cast `/Game/Blueprints/Character/BP_TDSCharacter` (`Controller.K2_GetPawn` _asbp_tdsplayer_controller)))
    (`/Engine/EditorBlueprintResources/StandardMacros.IsValid` _asbp_tdscharacter
      (:`Is Valid`
        (bind _output_get (set `self.TDSCharacterRef` _asbp_tdscharacter))
        (`/Game/Blueprints/UI/Inventory/WBP_InventoryStats.InitInventoryStatsWidget` (`/Game/Blueprints/UI/WBP_Gameplay.WBP_InventoryStats` _aswbp_gameplay) _output_get)
        (`TDS_GameplayWidget.Initialize` _aswbp_gameplay)))
    (else
      (`/Engine/EditorBlueprintResources/StandardMacros.IsValid` (`self.EndGameMenuReference`)
        (:`Is Valid`
          _)
        (:`Is Not Valid`
          (bind _returnvalue_2 (`|CreateWidget` "/Game/Blueprints/UI/Menu/WBP_EndGame.WBP_EndGame_C"))
          (set `self.EndGameMenuReference` _returnvalue_2)))
      (if (`GameplayStatics.IsGamePaused`)
        (`Widget.RemoveFromParent` _endgamemenureference)
        (`GameplayStatics.SetGamePaused` false)
        (set `PlayerController.bShowMouseCursor` false _returnvalue)
        (`WidgetBlueprintLibrary.SetInputMode_GameOnly` _returnvalue)
        (else
          (`UserWidget.AddToViewport` _endgamemenureference 0)
          (`GameplayStatics.SetGamePaused` true)
          (set `PlayerController.bShowMouseCursor` true _returnvalue)
          (`WidgetBlueprintLibrary.SetInputMode_GameAndUIEx` _returnvalue (`self.EndGameMenuReference`) "LockInFullscreen" false))))))

(fn `UserConstructionScript`
  (bind _cameraboom (`self.CameraBoom`))
  (set `SpringArmComponent.TargetArmLength` (`self.CameraHeightMax`) _cameraboom)
  (`SceneComponent.K2_SetRelativeRotation` _cameraboom (`self.RotatorCamera`) false false)
  (set `SpringArmComponent.bEnableCameraLag` (`self.Flow`) _cameraboom)
  (set `SpringArmComponent.CameraLagSpeed` (`self.CoefficientSmooth`) _cameraboom)
  (`SkinnedMeshComponent.SetLeaderPoseComponent` (`self.SK_ShellMannequin`) (`self.Mesh`) false))