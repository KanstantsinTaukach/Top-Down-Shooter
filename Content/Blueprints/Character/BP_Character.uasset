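; Top-down character Blueprint that handles camera behavior, a sprint trail and hotkeys for rifle fire, death montage and camera shake.
; Construction configures the camera boom's height, rotation and lag.
; Each tick feeds sprint velocity to a Niagara trail and, while aiming, slides the boom toward a distant cursor up to a zoom-scaled limit.
; The boom eases back to the character when not aiming or the cursor is near.
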(event `Key|F`
  (params (Key :type "Key Structure"))
  (:`Pressed`
    (`self.CameraShakeEvent`)))

(event `Key|SpaceBar`
  (params (Key :type "Key Structure"))
  (bind _mesh (`self.Mesh`))
  (:`Pressed`
    (if (`|EnumEquality` (`self.MovementState`) "Aim_State")
      (`|PlayMontage` _mesh "/Game/Blueprints/Character/Mannequin/Animations/TDSAnimations/AM_Fire_Rifle_Ironsights.AM_Fire_Rifle_Ironsights")
      (else
        (`|PlayMontage` _mesh "/Game/Blueprints/Character/Mannequin/Animations/TDSAnimations/AM_Fire_Rifle_Hip.AM_Fire_Rifle_Hip")))))

(event `Key|V`
  (params (Key :type "Key Structure"))
  (:`Pressed`
    (`|PlayMontage` (`self.Mesh`) "/Game/Blueprints/Character/Mannequin/Animations/TDSAnimations/AM_Death_1.AM_Death_1")))

(event `self.ReceiveTick`
  (params (DeltaSeconds :type "Float (single-precision)"))
  (`self.SetNiagaraTrail`)
  (`self.CameraSlideToCursor` DeltaSeconds))

(fn `CameraShakeEvent`
  (`GameplayStatics.PlayWorldCameraShake` "/Game/Blueprints/Game/BP_ShakeCamera.BP_ShakeCamera_C" (`SceneComponent.K2_GetComponentLocation` (`self.TopDownCameraComponent`)) 0.0 30.0))

(fn `CameraSlideToCursor`
  (params (InputPin :type "Float (double-precision)"))
  (bind _cameraboom (`self.CameraBoom`))
  (bind _returnvalue (`SceneComponent.K2_GetComponentLocation` (`self.CapsuleComponent`)))
  (bind (_returnvalue_x _returnvalue_y _returnvalue_z) (`KismetMathLibrary.BreakVector` (`SceneComponent.K2_GetComponentLocation` (`self.CameraBoom`))))
  (bind _returnvalue_2 (`self.GetCursorToWorld`))
  (set `self.ClampedCameraHeight` (`KismetMathLibrary.MapRangeClamped` (`SpringArmComponent.TargetArmLength` (`self.CameraBoom`)) (`self.CameraHeightMin`) (`self.CameraHeightMax`) 0.5 1.0))
  (bind _returnvalue_3 (`SceneComponent.K2_GetComponentLocation` _returnvalue_2))
  (set `self.DistanceCameraBoomChar` (`KismetMathLibrary.VSizeXY` (- _returnvalue _returnvalue_3)))
  (if (`|EnumEquality` (`self.MovementState`) "Aim_State")
    (if (> (`self.DistanceCameraBoomChar`) (* (`self.ClampedCameraHeight`) (`self.FMinClampDistanceLogicMouseCursorStart`)))
      (if (not (> (`KismetMathLibrary.VSize2D` (`KismetMathLibrary.Conv_VectorToVector2D` (- (`SceneComponent.K2_GetComponentLocation` (`self.CameraBoom`)) _returnvalue))) (* (`self.ClampedCameraHeight`) (`self.FMaxClampDistanceLogicMouseCursorStart`))))
        (bind (_x _y) (`KismetMathLibrary.BreakVector2D` (* (`KismetMathLibrary.Normal2D` (`KismetMathLibrary.Conv_VectorToVector2D` (`KismetMathLibrary.GetForwardVector` (`KismetMathLibrary.FindLookAtRotation` _returnvalue _returnvalue_3)))) (`self.FSpeedChangeLocationCameraToCursor`))))
        (`SceneComponent.K2_SetWorldLocation` (`self.CameraBoom`) (`KismetMathLibrary.MakeVector` (+ _x _returnvalue_x) (+ _y _returnvalue_y) _returnvalue_z) false false))
      (else
        (`SceneComponent.K2_SetWorldLocation` _cameraboom (`KismetMathLibrary.VInterpTo` (`SceneComponent.K2_GetComponentLocation` _cameraboom) (`SceneComponent.K2_GetComponentLocation` (`self.CapsuleComponent`)) InputPin (`self.FSpeedReturnCameraDefaultPosition`)) false false :!label _label)))
    (else
      (goto _label))))

(fn `SetNiagaraTrail`
  (if (`self.IsSprinting` self)
    (`NiagaraComponent.SetVariableFloat` (`self.NS_Trail`) "Sprint" (`KismetMathLibrary.VSize` (`MovementComponent.Velocity` (`self.CharacterMovement`))))
    (else
      (`NiagaraComponent.SetVariableFloat` (`self.NS_Trail`) "Sprint" 0.0))))

(fn `UserConstructionScript`
  (bind _cameraboom (`self.CameraBoom`))
  (set `SpringArmComponent.TargetArmLength` (`self.CameraHeightMax`) _cameraboom)
  (`SceneComponent.K2_SetRelativeRotation` _cameraboom (`self.RotatorCamera`) false false)
  (set `SpringArmComponent.bEnableCameraLag` (`self.Flow`) _cameraboom)
  (set `SpringArmComponent.CameraLagSpeed` (`self.CoefficientSmooth`) _cameraboom))