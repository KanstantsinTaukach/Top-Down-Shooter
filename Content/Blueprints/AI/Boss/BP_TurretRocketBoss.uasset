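; Rocket turret for the AI boss that fires explosive missiles once the boss's health drops to 50 or below.
; A looping timer started on BeginPlay polls the owning boss's HealthComponent and plays the Shoot timeline.
; The timeline's Shoot event spawns a missile at the Arrow component and initializes it with inline radial-damage, mesh and effect settings.
; When the boss's health is depleted, the turret clears the timer and destroys itself.
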(event `self.ReceiveBeginPlay`
  (bind _returnvalue (`KismetSystemLibrary.K2_SetTimerDelegate` (delegate `FireRocket`) 3.0 true))
  (set `self.FireRocketTimerHandle` _returnvalue))

(event `FireRocket`
  (bind _returnvalue (`self.GetOwner`))
  (bind _arrow (`self.Arrow`))
  (bind _asbp_tdsaicharacter_boss (cast `/Game/Blueprints/AI/Boss/BP_TDSAICharacter_Boss` _returnvalue))
  (bind _returnvalue_2 (`TDSHealthComponent.GetCurrentHealth` (`TDSAICharacterBase.HealthComponent` _asbp_tdsaicharacter_boss)))
  (if (> _returnvalue_2 0.0)
    (if (<= _returnvalue_2 50.0)
      (`Timeline|Shoot` :!via `PlayFromStart`
        (:`ShootEvent`
          (bind _returnvalue_3 (`|SpawnActorFromClass` "/Game/Blueprints/AI/Boss/BP_MissileTurret.BP_MissileTurret_C" (`KismetMathLibrary.MakeTransform` (+ (`SceneComponent.GetForwardVector` _arrow) (`SceneComponent.K2_GetComponentLocation` _arrow)) (`SceneComponent.K2_GetComponentRotation` _arrow)) "AlwaysSpawn" "OverrideRootScale" _returnvalue null))
          (`TDS_ProjectileDefault.InitProjectile` _returnvalue_3 (make `ProjectileInfo` :`Projectile` "/Game/Blueprints/AI/Boss/BP_MissileTurret.BP_MissileTurret_C" :`ProjectileStaticMesh` "/Game/Blueprints/AI/Boss/RocketLauncher/Rocket_Launcher_Rocket.Rocket_Launcher_Rocket" :`ProjectileStaticMeshOffset` (`KismetMathLibrary.MakeTransform` (65.0 -26.0 -2.0) (struct :`Pitch` 90.0 :`Roll` 90.0) (3.0 3.0 3.0)) :`ProjectileTrailFX` "/Game/Items/MilitaryWeapons/FX/P_RocketLauncher_Trail_01.P_RocketLauncher_Trail_01" :`ProjectileDamage` 0.0 :`ProjectileInitSpeed` 1200.0 :`ExplosiveProjectile` true :`ExplodeDecal` "/Game/Blueprints/Decals/ConcreteDamage/M_Decal_ConcreteDamage.M_Decal_ConcreteDamage" :`ExplodeFX` "/Game/Items/MilitaryWeapons/FX/P_RocketLauncher_Explosion_01.P_RocketLauncher_Explosion_01" :`ExplodeSound` "/Game/Items/MilitaryWeapons/Sound/RocketLauncher/RocketLauncher_Explosion_Cue.RocketLauncher_Explosion_Cue" :`ProjectileMaxRadiusDamage` 300.0 :`ProjectileMinRadiusDamage` 100.0 :`ExplodeMaxDamage` 30.0)))))
    (else
      (`KismetSystemLibrary.K2_ClearAndInvalidateTimerHandle` (`self.FireRocketTimerHandle`))
      (`self.K2_DestroyActor` self))))

(fn `UserConstructionScript`)