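; Base AI controller that turns perception updates about Player-tagged actors into blackboard data.
; Each update caches the actor as CurrentTarget, then branches on the stimulus sense class.
; Any hearing update writes the target's actual location, not the stimulus location, to LastTargetVector and sets CanHearTarget.
; Losing another sense writes that location and clears CanHearTarget, while successful non-hearing senses only update CurrentTarget.
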(event `self.TDSAIPerceptionComponent.OnTargetPerceptionUpdated`
  (params (Actor :type "Actor Object Reference") (Stimulus :type "AIStimulus Structure"))
  (bind _returnvalue (`AIBlueprintHelperLibrary.GetBlackboard` null))
  (bind _returnvalue_2 (`AIBlueprintHelperLibrary.GetBlackboard` null))
  (if (`self.ActorHasTag` Actor "Player")
    (set `self.CurrentTarget` Actor)
    (bind _returnvalue_3 (`AIPerceptionSystem.GetSenseClassForStimulus` Stimulus))
    (if (== _returnvalue_3 "/Script/AIModule.AISense_Hearing")
      (`BlackboardComponent.SetValueAsVector` _returnvalue_2 "LastTargetVector" (`self.K2_GetActorLocation` (`self.CurrentTarget`)))
      (`BlackboardComponent.SetValueAsBool` _returnvalue_2 "CanHearTarget" true)
      (elif (not (`.bSuccessfullySensed` (break `AIStimulus` Stimulus)))
        (`/Engine/EditorBlueprintResources/StandardMacros.IsValid` (`self.CurrentTarget`)
          (:`Is Valid`
            (`BlackboardComponent.SetValueAsVector` _returnvalue "LastTargetVector" (`self.K2_GetActorLocation` (`self.CurrentTarget`)))
            (`BlackboardComponent.SetValueAsBool` _returnvalue "CanHearTarget" false)))))))

(fn `UserConstructionScript`)