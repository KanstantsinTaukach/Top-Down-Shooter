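; AI controller for TDS enemies that turns perception updates about Player-tagged actors into Blackboard values.
; Hearing stimuli store the actor's location in LastTargetVector and set CanHearTarget, which is never cleared here.
; Other senses set TargetActor and CanSeeTarget when sensed, and clear both when lost.
; Losing the target also draws a debug sphere and label at the actor's current location.
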(event `self.AIPerception.OnTargetPerceptionUpdated`
  (params (Actor :type "Actor Object Reference") (Stimulus :type "AIStimulus Structure"))
  (bind _returnvalue (`AIBlueprintHelperLibrary.GetBlackboard` null))
  (bind _returnvalue_2 (`AIBlueprintHelperLibrary.GetBlackboard` null))
  (bind _returnvalue_3 (`AIBlueprintHelperLibrary.GetBlackboard` null))
  (bind _returnvalue_4 (`self.K2_GetActorLocation` (`self.CurrentTarget`)))
  (set `self.CurrentTarget` Actor)
  (if (`self.ActorHasTag` Actor "Player")
    (bind _returnvalue_5 (`AIPerceptionSystem.GetSenseClassForStimulus` Stimulus))
    (if (== _returnvalue_5 "/Script/AIModule.AISense_Hearing")
      (`BlackboardComponent.SetValueAsVector` _returnvalue "LastTargetVector" (`self.K2_GetActorLocation` (`self.CurrentTarget`)))
      (`BlackboardComponent.SetValueAsBool` _returnvalue "CanHearTarget" true)
      (elif (`.bSuccessfullySensed` (break `AIStimulus` Stimulus))
        (`BlackboardComponent.SetValueAsObject` _returnvalue_2 "TargetActor" (`self.CurrentTarget`))
        (`BlackboardComponent.SetValueAsBool` _returnvalue_2 "CanSeeTarget" true)
        (else
          (`/Engine/EditorBlueprintResources/StandardMacros.IsValid` (`self.CurrentTarget`)
            (:`Is Valid`
              (`BlackboardComponent.SetValueAsObject` _returnvalue_3 "TargetActor" null)
              (`BlackboardComponent.SetValueAsBool` _returnvalue_3 "CanSeeTarget" false)
              (`KismetSystemLibrary.DrawDebugSphere` _returnvalue_4 20.0 12 (struct :`R` 1.0 :`G` 0.116532 :`A` 1.0) 10.0)
              (`KismetSystemLibrary.DrawDebugString` _returnvalue_4 "I lost target here" null (struct :`G` 1.0 :`B` 0.238495 :`A` 1.0) 10.0))
            (:`Is Not Valid`
              (`KismetSystemLibrary.PrintString` "Target Perception: Current Target is not valid!" true true (struct :`R` 1.0 :`G` 0.037429 :`A` 1.0) 10.0))))))))

(fn `UserConstructionScript`)