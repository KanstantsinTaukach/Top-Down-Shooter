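; AI controller for the Parasite enemy that turns perception updates into blackboard keys.
; Stimuli tagged as an airborne grenade set the grenade target, whatever the actor.
; For player-tagged actors, hearing records the last location and flags the target as heard.
; Other senses set the target actor when sensed and clear it on a failed stimulus if a current target is valid.
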(event `self.AIPerception.OnTargetPerceptionUpdated`
  (params (Actor :type "Actor Object Reference") (Stimulus :type "AIStimulus Structure"))
  (bind _returnvalue (`AIBlueprintHelperLibrary.GetBlackboard` null))
  (if (== (`.Tag` (break `AIStimulus` Stimulus)) "GrenadeInAir")
    (bind _output_get (set `self.CurrentTarget` Actor))
    (`BlackboardComponent.SetValueAsObject` (`AIBlueprintHelperLibrary.GetBlackboard` null) "TargetGrenade" _output_get)
    (elif (`self.ActorHasTag` Actor "Player")
      (set `self.CurrentTarget` Actor)
      (bind _returnvalue_2 (`AIPerceptionSystem.GetSenseClassForStimulus` Stimulus))
      (if (== _returnvalue_2 "/Script/AIModule.AISense_Hearing")
        (`BlackboardComponent.SetValueAsVector` _returnvalue "LastTargetVector" (`self.K2_GetActorLocation` (`self.CurrentTarget`)))
        (`BlackboardComponent.SetValueAsBool` _returnvalue "CanHearTarget" true)
        (elif (`.bSuccessfullySensed` (break `AIStimulus` Stimulus))
          (`BlackboardComponent.SetValueAsObject` (`AIBlueprintHelperLibrary.GetBlackboard` null) "TargetActor" (`self.CurrentTarget`))
          (else
            (`/Engine/EditorBlueprintResources/StandardMacros.IsValid` (`self.CurrentTarget`)
              (:`Is Valid`
                (`BlackboardComponent.SetValueAsObject` (`AIBlueprintHelperLibrary.GetBlackboard` null) "TargetActor" null)))))))))

(fn `UserConstructionScript`)