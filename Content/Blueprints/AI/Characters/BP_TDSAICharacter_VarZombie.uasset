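; Zombie variant of the top-down-shooter AI character that chases the player and shows feedback when hurt.
; Every tick it searches for all BP_TDSCharacter actors and issues a simple move toward the first valid one.
; When its HealthComponent reports damage, it spawns a BP_DisplayDamageActor at a randomly jittered offset from its location, initialized with current health and damage taken.
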(event `self.HealthComponent.OnTakeDamage`
  (params (Health :type "Float (single-precision)") (Damage :type "Float (single-precision)"))
  (bind _returnvalue (`|SpawnActorFromClass` "/Game/Blueprints/InteractionEnvironment/MadeOnBlueprints/BP_DisplayDamageActor.BP_DisplayDamageActor_C" (`KismetMathLibrary.Conv_VectorToTransform` (+ (`self.K2_GetActorLocation`) (+ (`KismetMathLibrary.MakeVector` (`KismetMathLibrary.RandomFloatInRange` -20.0 20.0) (`KismetMathLibrary.RandomFloatInRange` -20.0 20.0)) (/ (`KismetMathLibrary.Conv_DoubleToVector` (.z (`self.K2_GetActorLocation`))) 3.0)))) "AlwaysSpawn" "OverrideRootScale" null null))
  (`/Game/Blueprints/InteractionEnvironment/MadeOnBlueprints/BP_DisplayDamageActor.InitActor` _returnvalue Health Damage))

(event `self.ReceiveTick`
  (params (DeltaSeconds :type "Float (single-precision)"))
  (bind _outactors (`GameplayStatics.GetAllActorsOfClass` "/Game/Blueprints/Character/BP_TDSCharacter.BP_TDSCharacter_C"))
  (bind _output (`|GetArrayItem` _outactors))
  (`/Engine/EditorBlueprintResources/StandardMacros.IsValid` _output
    (:`Is Valid`
      (`AIBlueprintHelperLibrary.SimpleMoveToActor` (`self.GetController`) _output))))

(fn `UserConstructionScript`)