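; Base enemy character that takes damage, shows damage numbers and handles its own death.
; Point damage feeds HealthComponent, whose damage event spawns a randomly offset BP_DisplayDamageActor.
; On death it unpossesses, blocks movement and attack, disables capsule collision, sets a lifespan, and plays a random death montage before switching the mesh to physics.
; Radial damage is unhandled: its damage and surface-effect logic is disconnected.
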(event `self.HealthComponent.OnTakeDamage`
  (params (Health :type "Float (single-precision)") (Damage :type "Float (single-precision)"))
  (bind _returnvalue (`|SpawnActorFromClass` "/Game/Blueprints/InteractionEnvironment/MadeOnBlueprints/BP_DisplayDamageActor.BP_DisplayDamageActor_C" (`KismetMathLibrary.Conv_VectorToTransform` (+ (`self.K2_GetActorLocation`) (+ (`KismetMathLibrary.MakeVector` (`KismetMathLibrary.RandomFloatInRange` -20.0 20.0) (`KismetMathLibrary.RandomFloatInRange` -20.0 20.0)) (/ (`KismetMathLibrary.Conv_DoubleToVector` (.z (`self.K2_GetActorLocation`))) 3.0)))) "AlwaysSpawn" "OverrideRootScale" null null))
  (`/Game/Blueprints/InteractionEnvironment/MadeOnBlueprints/BP_DisplayDamageActor.InitActor` _returnvalue Health Damage))

(event `self.ReceivePointDamage`
  (params (Damage :type "Float (single-precision)") (DamageType :type "DamageType Object Reference") (HitLocation :type "Vector Structure") (HitNormal :type "Vector Structure") (HitComponent :type "PrimitiveComponent Object Reference") (BoneName :type Name) (ShotFromDirection :type "Vector Structure") (InstigatedBy :type "Controller Object Reference") (DamageCauser :type "Actor Object Reference") (HitInfo :type "HitResult Structure (by ref)"))
  (if (not (`self.bIsDead`))
    (`TDSHealthComponent.RemoveFromCurrentHealth` (`self.HealthComponent`) Damage)))

(event `self.ReceiveRadialDamage`
  (params (DamageReceived :type "Float (single-precision)") (DamageType :type "DamageType Object Reference") (Origin :type "Vector Structure") (HitInfo :type "HitResult Structure (by ref)") (InstigatedBy :type "Controller Object Reference") (DamageCauser :type "Actor Object Reference")))

(event `self.HealthComponent.OnDeath`
  (bind _mesh (`self.Mesh`))
  (bind _outitem (`KismetArrayLibrary.Array_Random` (`self.DeadsAnimation`)))
  (`self.EnemyDead`)
  (`PrimitiveComponent.SetCollisionEnabled` (`self.CapsuleComponent`) "NoCollision")
  (`/Engine/EditorBlueprintResources/StandardMacros.IsValid` _outitem
    (:`Is Valid`
      (`|PlayMontage` (`self.Mesh`) _outitem
        (:`OnCompleted`
          (`PrimitiveComponent.SetCollisionEnabled` _mesh "PhysicsOnly")
          (`PrimitiveComponent.SetCollisionProfileName` _mesh "PhysicsActor" true)
          (`PrimitiveComponent.SetSimulatePhysics` _mesh true))))))

(fn `EnemyDead`
  (`Controller.UnPossess` (`self.GetController`))
  (`self.SetMovementState` false)
  (`self.SetAttackState` false)
  (`self.SetLifeSpan` 10.0)
  (set `self.bIsDead` true))

(fn `SetAttackState`
  (params (CanAttack :type Boolean))
  (set `self.CanAttack` CanAttack))

(fn `SetMovementState`
  (params (CanMove :type Boolean))
  (set `self.CanMove` CanMove))

(fn `UserConstructionScript`)